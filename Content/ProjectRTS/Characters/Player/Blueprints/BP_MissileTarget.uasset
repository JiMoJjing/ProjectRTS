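; BP_MissileTarget is a missile target marker actor that orients itself and shows a lock-on effect.
; LockOnEffectActivate turns it to face away from its owner's location on an enemy hit, or along the hit normal otherwise, then activates LockOnEffect with reset.
; An enemy hit without a valid owner does nothing, and the event graph and construction script are empty, so activation relies on an external call.
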(fn `LockOnEffectActivate`
  (params (InHitNormal :type "Vector Structure") (bIsHitEnemy :type Boolean))
  (bind _returnvalue (`self.GetOwner`))
  (if bIsHitEnemy
    (`/Engine/EditorBlueprintResources/StandardMacros.IsValid` _returnvalue
      (:`Is Valid`
        (`self.K2_SetActorRotation` (`KismetMathLibrary.FindLookAtRotation` (`self.K2_GetActorLocation` _returnvalue) (`self.K2_GetActorLocation`)))
        (`ActorComponent.Activate` (`self.LockOnEffect`) true)))
    (else
      (`self.K2_SetActorRotation` (`KismetMathLibrary.Conv_VectorToRotator` InHitNormal))
      (`ActorComponent.Activate` (`self.LockOnEffect`) true))))

(fn `UserConstructionScript`)