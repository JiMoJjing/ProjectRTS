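; Player missile projectile that explodes on contact and deals area damage.
; On spawn it sets a lifespan and a timer that turns on homing after a delay, if the projectile movement already has a valid target.
; A sphere hit or overlap spawns a small Niagara explosion, applies random full radial damage credited to the instigator's controller, then destroys the missile.
; An older sphere-trace damage chain remains unconnected.
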(event `self.ReceiveBeginPlay`
  (`KismetSystemLibrary.K2_SetTimerDelegate` (delegate `HomingStart`) (`self.HomingStartTime`))
  (`self.SetLifeSpan` (`self.LifeTime`)))

(event `HomingStart`
  (bind _projectilemovement (`self.ProjectileMovement`))
  (`ProjectileMovementComponent.HomingTargetComponent` _projectilemovement
    (:`then`
      (set `ProjectileMovementComponent.bIsHomingProjectile` true _projectilemovement))
    (:`else`)))

(event `self.Sphere.OnComponentHit`
  (params (HitComponent :type "PrimitiveComponent Object Reference") (OtherActor :type "Actor Object Reference") (OtherComp :type "PrimitiveComponent Object Reference") (NormalImpulse :type "Vector Structure") (Hit :type "HitResult Structure (by ref)"))
  (`NiagaraFunctionLibrary.SpawnSystemAtLocation` (`self.ExplosionNiagaraEffect`) (`self.K2_GetActorLocation`) (struct) (0.1 0.1 0.1))
  (`GameplayStatics.ApplyRadialDamage` :`BaseDamage` (`KismetMathLibrary.RandomFloatInRange` (`self.MissileDamageMin`) (`self.MissileDamageMax`)) :`Origin` (`self.K2_GetActorLocation`) :`DamageRadius` (`self.ExplosionRadius`) :`DamageCauser` self :`InstigatedByController` (`Pawn.GetController` (`self.Instigator`)) :`bDoFullDamage` true :!label _label)
  (`self.K2_DestroyActor`))

(event `self.Sphere.OnComponentBeginOverlap`
  (params (OverlappedComponent :type "PrimitiveComponent Object Reference") (OtherActor :type "Actor Object Reference") (OtherComp :type "PrimitiveComponent Object Reference") (OtherBodyIndex :type Integer) (bFromSweep :type Boolean) (SweepResult :type "HitResult Structure (by ref)"))
  (`NiagaraFunctionLibrary.SpawnSystemAtLocation` (`self.ExplosionNiagaraEffect`) (`self.K2_GetActorLocation`) (struct) (0.1 0.1 0.1))
  (goto _label))

(fn `UserConstructionScript`)