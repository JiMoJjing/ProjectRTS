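; BP_Mushroom is an enemy that reacts to player damage with hit feedback and floating damage numbers; no health handling appears here.
; Point and radial damage events report to the instigator's pawn through IApplyDamageFeedback, with head-bone hits doubled and flagged as critical.
; Each hit spawns NS_DamageNumbers, passing position and amount in one Vector4 array and scaling sprite size by instigator distance.
; The pushback and fire reactions in the Deplicated graph never run.
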(event `self.ReceiveRadialDamage`
  (params (DamageReceived :type "Float (single-precision)") (DamageType :type "DamageType Object Reference") (Origin :type "Vector Structure") (HitInfo :type "HitResult Structure (by ref)") (InstigatedBy :type "Controller Object Reference") (DamageCauser :type "Actor Object Reference"))
  (bind _returnvalue (`Controller.K2_GetPawn` InstigatedBy))
  (bind (_damageeffectsizemin_x _damageeffectsizemin_y) (`KismetMathLibrary.BreakVector2D` (`self.DamageEffectSizeMin`)))
  (bind (_damageeffectsizemax_x _damageeffectsizemax_y) (`KismetMathLibrary.BreakVector2D` (`self.DamageEffectSizeMax`)))
  (bind _returnvalue_2 (/ (`KismetMathLibrary.Vector_Distance2D` (`self.K2_GetActorLocation`) (`self.K2_GetActorLocation` _returnvalue)) (`self.DamageEffectRenderDistanceMax`)))
  (bind _asiapply_damage_feedback (cast `/Game/ProjectRTS/Interface/IApplyDamageFeedback` _returnvalue))
  (`/Game/ProjectRTS/Interface/IApplyDamageFeedback.ApplyDamageFeedback` _asiapply_damage_feedback DamageReceived false)
  (bind _returnvalue_3 (`NiagaraFunctionLibrary.SpawnSystemAtLocation` "/Game/ProjectRTS/VFX/NS_DamageNumbers.NS_DamageNumbers"))
  (`NiagaraDataInterfaceArrayFunctionLibrary.SetNiagaraArrayVector4` _returnvalue_3 "User.DamageInfo" (`|MakeArray` (`KismetMathLibrary.MakeVector4` (.x (`self.GetRandomDamageEffectLocation`)) (.y (`self.GetRandomDamageEffectLocation`)) (.z (`self.GetRandomDamageEffectLocation`)) DamageReceived)))
  (`NiagaraComponent.SetVariableVec2` _returnvalue_3 "User.SpriteSize" (`KismetMathLibrary.MakeVector2D` (`KismetMathLibrary.Lerp` _damageeffectsizemin_x _damageeffectsizemax_x _returnvalue_2) (`KismetMathLibrary.Lerp` _damageeffectsizemin_y _damageeffectsizemax_y _returnvalue_2))))

(event `self.ReceivePointDamage`
  (params (Damage :type "Float (single-precision)") (DamageType :type "DamageType Object Reference") (HitLocation :type "Vector Structure") (HitNormal :type "Vector Structure") (HitComponent :type "PrimitiveComponent Object Reference") (BoneName :type Name) (ShotFromDirection :type "Vector Structure") (InstigatedBy :type "Controller Object Reference") (DamageCauser :type "Actor Object Reference") (HitInfo :type "HitResult Structure (by ref)"))
  (bind _returnvalue (`Controller.K2_GetPawn` InstigatedBy))
  (bind (_damageeffectsizemin_x _damageeffectsizemin_y) (`KismetMathLibrary.BreakVector2D` (`self.DamageEffectSizeMin`)))
  (bind (_damageeffectsizemax_x _damageeffectsizemax_y) (`KismetMathLibrary.BreakVector2D` (`self.DamageEffectSizeMax`)))
  (bind _returnvalue_2 (== BoneName (`self.HeadBoneName`)))
  (bind _returnvalue_3 (/ (`KismetMathLibrary.Vector_Distance` (`self.K2_GetActorLocation`) (`self.K2_GetActorLocation` _returnvalue)) (`self.DamageEffectRenderDistanceMax`)))
  (bind _asiapply_damage_feedback (cast `/Game/ProjectRTS/Interface/IApplyDamageFeedback` _returnvalue))
  (if _returnvalue_2
    (set `self.Damage` (* Damage 2.0))
    (else
      (set `self.Damage` Damage)))
  (`/Game/ProjectRTS/Interface/IApplyDamageFeedback.ApplyDamageFeedback` _asiapply_damage_feedback (`self.Damage`) _returnvalue_2)
  (bind _returnvalue_4 (`NiagaraFunctionLibrary.SpawnSystemAtLocation` "/Game/ProjectRTS/VFX/NS_DamageNumbers.NS_DamageNumbers"))
  (`NiagaraDataInterfaceArrayFunctionLibrary.SetNiagaraArrayVector4` _returnvalue_4 "User.DamageInfo" (`|MakeArray` (`KismetMathLibrary.MakeVector4` (.x (`self.GetRandomDamageEffectLocation`)) (.y (`self.GetRandomDamageEffectLocation`)) (.z (`self.GetRandomDamageEffectLocation`)) (`KismetMathLibrary.Conv_IntToDouble` (`KismetMathLibrary.FFloor` (`self.Damage`))))))
  (`NiagaraComponent.SetVariableBool` _returnvalue_4 "User.Critical" _returnvalue_2)
  (`NiagaraComponent.SetVariableVec2` _returnvalue_4 "User.SpriteSize" (`KismetMathLibrary.MakeVector2D` (`KismetMathLibrary.Lerp` _damageeffectsizemin_x _damageeffectsizemax_x _returnvalue_3) (`KismetMathLibrary.Lerp` _damageeffectsizemin_y _damageeffectsizemax_y _returnvalue_3))))

(fn `UserConstructionScript`)